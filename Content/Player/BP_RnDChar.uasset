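; BP_RnDChar is a player character that creates the HUD, drives lockpicking and runs NPC dialog.
; Rotation axes forward to the interacted BP_Lock while it is active.
; EnterDialog pulls row data from the partner into W_DialogInterface, reusing up to five answer buttons carrying goto rows.
; Shoot reveals answers, steps listen-only lines until "end", or calls ExitDialog, whose InDialog reset is disconnected.
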(event `InputAxis|RotatePin`
  (params (AxisValue :type "Float (single-precision)"))
  (bind _interactedobject (`self.InteractedObject`))
  (bind _asbp_lock (cast `/Game/LockPicking/BP_Lock` _interactedobject :!pure true))
  ;[1 1 1] LockPicking
  (if (and (!= _interactedobject null) (== (`GameplayStatics.GetObjectClass` _interactedobject) "/Game/LockPicking/BP_Lock.BP_Lock_C"))
    (if (`/Game/LockPicking/BP_Lock.bIsActive` _asbp_lock)
      (`/Game/LockPicking/BP_Lock.RotatePin` _asbp_lock AxisValue))))

(event `InputAction|Shoot`
  (params (Key :type "Key Structure" :default "AnyKey"))
  ;[1 1 1] Shooting / Mouse Interact
  (:`Pressed`
    (if (`self.bInDialog`)
      (if (`self.bExit`)
        (`self.ExitDialog`)
        (elif (`DialogCharBase.bListenOnly` (cast `DialogCharBase` (`self.DialogPartner`) :!pure true))
          (`self.NextResponse`)
          (elif (`self.bResponeShowing`)
            (`self.ShowAnswers`)))))))

(event `InputAxis|RotateLock`
  (params (AxisValue :type "Float (single-precision)"))
  (bind _interactedobject (`self.InteractedObject`))
  (bind _asbp_lock (cast `/Game/LockPicking/BP_Lock` _interactedobject :!pure true))
  ;[1 1 1] LockPicking
  (if (and (!= _interactedobject null) (== (`GameplayStatics.GetObjectClass` _interactedobject) "/Game/LockPicking/BP_Lock.BP_Lock_C"))
    (if (`/Game/LockPicking/BP_Lock.bIsActive` _asbp_lock)
      (`/Game/LockPicking/BP_Lock.RotateLock` _asbp_lock AxisValue))))

(event `self.ReceiveBeginPlay`
  (bind _returnvalue (`|CreateWidget` "/Game/Player/W_PlayerHUD.W_PlayerHUD_C"))
  (`UserWidget.AddToViewport` _returnvalue 0))

(fn `EnterDialog`
  (params (DIalogPartner :type "Actor Object Reference"))
  (bind _row (`self.Row`))
  (set `self.DialogPartner` DIalogPartner)
  (set `self.Row` (`DialogCharBase.DialogStartRow` (cast `/Game/Dialog/BP_DialogBot` DIalogPartner :!pure true)))
  (set `self.bInDialog` true)
  (if (not (!= (`self.DialogInterface`) null))
    (bind _returnvalue (`|CreateWidget` "/Game/Dialog/W_DialogInterface.W_DialogInterface_C"))
    (bind _output_get (set `self.DialogInterface` _returnvalue)))
  (`TextBlock.SetText` (`/Game/Dialog/W_DialogInterface.NameText` _output_get) (`KismetTextLibrary.Conv_NameToText` (`DialogCharBase.CharacterName` (cast `/Game/Dialog/BP_DialogBot` (`self.DialogPartner`) :!pure true))))
  (`self.ShowResponse` _row)
  (if (not (`DialogCharBase.bListenOnly` (cast `DialogCharBase` (`self.DialogPartner`) :!pure true)))
    (`self.SetupAnswers` _row))
  (`UserWidget.AddToViewport` (`self.DialogInterface`) 0)
  (set `PlayerController.bShowMouseCursor` true (`GameplayStatics.GetPlayerController` 0)))

(fn `ExitDialog`
  (`Widget.RemoveFromParent` (`self.DialogInterface`))
  (set `self.bExit` false)
  (set `PlayerController.bShowMouseCursor` false (`GameplayStatics.GetPlayerController` 0)))

(fn `NextResponse`
  (bind _output_get (set `self.Row` (+ (`self.Row`) 1)))
  (bind _returnvalue (`DialogCharBase.getDialogRowData` (cast `DialogCharBase` (`self.DialogPartner`) :!pure true) _output_get))
  (if (`KismetTextLibrary.EqualEqual_TextText` (`.AnswerEnd` (break `DialogData` _returnvalue)) (`|FormatText` "end"))
    (`self.ShowResponse` _output_get)
    (set `self.bExit` true)
    (else
      (`self.ShowResponse` _output_get))))

(fn `SetupAnswers`
  (params (Row :type Integer))
  (bind _answer2 (`self.Answer2`))
  (bind _answer1 (`self.Answer1`))
  (bind _answer3 (`self.Answer3`))
  (bind _answer4 (`self.Answer4`))
  (bind _answerend (`self.AnswerEnd`))
  (bind _returnvalue (!= _answer3 null))
  (bind _returnvalue_2 (!= _answer4 null))
  (bind _returnvalue_3 (!= _answer1 null))
  (bind _returnvalue_4 (!= (`self.Answer2`) null))
  (bind _asbp_dialog_bot (cast `/Game/Dialog/BP_DialogBot` (`self.DialogPartner`)))
  (bind _returnvalue_5 (`DialogCharBase.getDialogRowData` _asbp_dialog_bot Row))
  (if (or (not (`KismetTextLibrary.TextIsEmpty` (`.Answer1` (break `DialogData` _returnvalue_5)))) (not (`KismetTextLibrary.TextIsEmpty` (`.Answer2` (break `DialogData` _returnvalue_5)))) (not (`KismetTextLibrary.TextIsEmpty` (`.Answer3` (break `DialogData` _returnvalue_5)))) (not (`KismetTextLibrary.TextIsEmpty` (`.Answer4` (break `DialogData` _returnvalue_5)))) (not (`KismetTextLibrary.TextIsEmpty` (`.AnswerEnd` (break `DialogData` _returnvalue_5)))))
    (`|ExecutionSequence`
      (:`then_0`
        (if (`KismetTextLibrary.TextIsEmpty` (`.Answer1` (break `DialogData` _returnvalue_5)))
          (if _returnvalue_3
            (`Widget.RemoveFromParent` _answer1))
          (elif _returnvalue_3
            (`TextBlock.SetText` (`/Game/Dialog/W_DialogButton.AnswerText` _answer1) (`.Answer1` (break `DialogData` _returnvalue_5)))
            (set `/Game/Dialog/W_DialogButton.changeto` (`.A1Goto` (break `DialogData` _returnvalue_5)) _answer1)
            (`Widget.RemoveFromParent` _answer1)
            (`PanelWidget.AddChild` (`/Game/Dialog/W_DialogInterface.AnswersBox` (`self.DialogInterface`)) _answer1)
            (else
              (bind _returnvalue_6 (`|CreateWidget` "/Game/Dialog/W_DialogButton.W_DialogButton_C"))
              (set `self.Answer1` _returnvalue_6)
              (`TextBlock.SetText` (`/Game/Dialog/W_DialogButton.AnswerText` _returnvalue_6) (`.Answer1` (break `DialogData` _returnvalue_5)))
              (`PanelWidget.AddChild` (`/Game/Dialog/W_DialogInterface.AnswersBox` (`self.DialogInterface`)) _returnvalue_6)
              (set `/Game/Dialog/W_DialogButton.changeto` (`.A1Goto` (break `DialogData` _returnvalue_5)) _returnvalue_6)))))
      (:`then_1`
        (if (`KismetTextLibrary.TextIsEmpty` (`.Answer2` (break `DialogData` _returnvalue_5)))
          (if _returnvalue_4
            (`Widget.RemoveFromParent` _answer2))
          (elif _returnvalue_4
            (`TextBlock.SetText` (`/Game/Dialog/W_DialogButton.AnswerText` _answer2) (`.Answer2` (break `DialogData` _returnvalue_5)))
            (set `/Game/Dialog/W_DialogButton.changeto` (`.A2Goto` (break `DialogData` _returnvalue_5)) _answer2)
            (`Widget.RemoveFromParent` _answer2)
            (`PanelWidget.AddChild` (`/Game/Dialog/W_DialogInterface.AnswersBox` (`self.DialogInterface`)) _answer2)
            (else
              (bind _returnvalue_7 (`|CreateWidget` "/Game/Dialog/W_DialogButton.W_DialogButton_C"))
              (set `self.Answer2` _returnvalue_7)
              (`TextBlock.SetText` (`/Game/Dialog/W_DialogButton.AnswerText` _returnvalue_7) (`.Answer2` (break `DialogData` _returnvalue_5)))
              (`PanelWidget.AddChild` (`/Game/Dialog/W_DialogInterface.AnswersBox` (`self.DialogInterface`)) _returnvalue_7)
              (set `/Game/Dialog/W_DialogButton.changeto` (`.A2Goto` (break `DialogData` _returnvalue_5)) _returnvalue_7)))))
      (:`then_2`
        (if (`KismetTextLibrary.TextIsEmpty` (`.Answer3` (break `DialogData` _returnvalue_5)))
          (if _returnvalue
            (`Widget.RemoveFromParent` _answer3))
          (elif _returnvalue
            (`TextBlock.SetText` (`/Game/Dialog/W_DialogButton.AnswerText` _answer3) (`.Answer3` (break `DialogData` _returnvalue_5)))
            (set `/Game/Dialog/W_DialogButton.changeto` (`.A3Goto` (break `DialogData` _returnvalue_5)) _answer3)
            (`Widget.RemoveFromParent` _answer3)
            (`PanelWidget.AddChild` (`/Game/Dialog/W_DialogInterface.AnswersBox` (`self.DialogInterface`)) _answer3)
            (else
              (bind _returnvalue_8 (`|CreateWidget` "/Game/Dialog/W_DialogButton.W_DialogButton_C"))
              (set `self.Answer3` _returnvalue_8)
              (`TextBlock.SetText` (`/Game/Dialog/W_DialogButton.AnswerText` _returnvalue_8) (`.Answer3` (break `DialogData` _returnvalue_5)))
              (`PanelWidget.AddChild` (`/Game/Dialog/W_DialogInterface.AnswersBox` (`self.DialogInterface`)) _returnvalue_8)
              (set `/Game/Dialog/W_DialogButton.changeto` (`.A3Goto` (break `DialogData` _returnvalue_5)) _returnvalue_8)))))
      (:`then_3`
        (if (`KismetTextLibrary.TextIsEmpty` (`.Answer4` (break `DialogData` _returnvalue_5)))
          (if _returnvalue_2
            (`Widget.RemoveFromParent` _answer4))
          (elif _returnvalue_2
            (`TextBlock.SetText` (`/Game/Dialog/W_DialogButton.AnswerText` _answer4) (`.Answer4` (break `DialogData` _returnvalue_5)))
            (set `/Game/Dialog/W_DialogButton.changeto` (`.A4Goto` (break `DialogData` _returnvalue_5)) _answer4)
            (`Widget.RemoveFromParent` _answer4)
            (`PanelWidget.AddChild` (`/Game/Dialog/W_DialogInterface.AnswersBox` (`self.DialogInterface`)) _answer4)
            (else
              (bind _returnvalue_9 (`|CreateWidget` "/Game/Dialog/W_DialogButton.W_DialogButton_C"))
              (set `self.Answer4` _returnvalue_9)
              (`TextBlock.SetText` (`/Game/Dialog/W_DialogButton.AnswerText` _returnvalue_9) (`.Answer4` (break `DialogData` _returnvalue_5)))
              (`PanelWidget.AddChild` (`/Game/Dialog/W_DialogInterface.AnswersBox` (`self.DialogInterface`)) _returnvalue_9)
              (set `/Game/Dialog/W_DialogButton.changeto` (`.A4Goto` (break `DialogData` _returnvalue_5)) _returnvalue_9)))))
      (:`then_4`
        (if (!= _answerend null)
          (if (not (`KismetTextLibrary.TextIsEmpty` (`.AnswerEnd` (break `DialogData` _returnvalue_5))))
            (`TextBlock.SetText` (`/Game/Dialog/W_DialogButton.AnswerText` _answerend) (`.AnswerEnd` (break `DialogData` _returnvalue_5))))
          (`Widget.RemoveFromParent` _answerend)
          (`PanelWidget.AddChild` (`/Game/Dialog/W_DialogInterface.AnswersBox` (`self.DialogInterface`)) _answerend)
          (else
            (bind _returnvalue_10 (`|CreateWidget` "/Game/Dialog/W_DialogButton.W_DialogButton_C"))
            (set `self.AnswerEnd` _returnvalue_10)
            (`TextBlock.SetText` (`/Game/Dialog/W_DialogButton.AnswerText` _returnvalue_10) (`.AnswerEnd` (break `DialogData` _returnvalue_5)))
            (`PanelWidget.AddChild` (`/Game/Dialog/W_DialogInterface.AnswersBox` (`self.DialogInterface`)) _returnvalue_10)
            (set `/Game/Dialog/W_DialogButton.changeto` -1 _returnvalue_10)))))))

(fn `ShowAnswers`
  (bind _dialoginterface (`self.DialogInterface`))
  (`Widget.SetVisibility` (`/Game/Dialog/W_DialogInterface.SubtitlesText` _dialoginterface) "Hidden")
  (`Widget.SetVisibility` (`/Game/Dialog/W_DialogInterface.AnswersBox` _dialoginterface) "Visible")
  (set `self.bResponeShowing` false))

(fn `ShowResponse`
  (params (Row :type Integer))
  (bind _dialoginterface (`self.DialogInterface`))
  (bind _subtitlestext (`/Game/Dialog/W_DialogInterface.SubtitlesText` _dialoginterface))
  (bind _asbp_dialog_bot (cast `/Game/Dialog/BP_DialogBot` (`self.DialogPartner`)))
  (bind _returnvalue (`DialogCharBase.getDialogRowData` _asbp_dialog_bot Row))
  (`TextBlock.SetText` _subtitlestext (break `DialogData` _returnvalue))
  (`Widget.SetVisibility` (`/Game/Dialog/W_DialogInterface.AnswersBox` _dialoginterface) "Hidden")
  (`Widget.SetVisibility` _subtitlestext "Visible")
  (set `self.bResponeShowing` true))

(fn `UserConstructionScript`)